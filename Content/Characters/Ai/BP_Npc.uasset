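; BP_Npc is an AI character with normal, investigate and combat alert states.
; Each state event sets a walk speed, prints AlertAcc as debug text and shows or hides a WB_Alertness widget, passing it the investigate or combat state.
; Tick feeds AlertAcc to the widget's radial progress and reapplies the normal patrol state whenever it equals zero; this graph never changes AlertAcc itself.
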(event `SetStateCombat`
  (`KismetSystemLibrary.PrintString` (`KismetStringLibrary.Conv_DoubleToString` (`self.AlertAcc`)) true true (struct :`R` 1.0 :`A` 1.0) 0.01)
  (set `CharacterMovementComponent.MaxWalkSpeed` (`self.SpeedCombat`) (`self.CharacterMovement`))
  (bind _aswb_alertness (cast `/Game/Characters/Ai/WB_Alertness` (`WidgetComponent.GetWidget` (`self.Widget`))))
  (`/Game/Characters/Ai/WB_Alertness.StateManager` _aswb_alertness "Combat")
  (`SceneComponent.SetVisibility` (`self.Widget`) true true))

(event `self.ReceiveBeginPlay`
  (`self.SetStateNormal`))

(event `SetStateInvestigate`
  (bind _alertacc (`self.AlertAcc`))
  (if (> _alertacc 0.0)
    (`KismetSystemLibrary.PrintString` (`KismetStringLibrary.Conv_DoubleToString` _alertacc) true true (struct :`R` 1.0 :`G` 0.6 :`A` 1.0) 0.01)
    (set `CharacterMovementComponent.MaxWalkSpeed` (`self.SpeedInvestigation`) (`self.CharacterMovement`))
    (bind _aswb_alertness (cast `/Game/Characters/Ai/WB_Alertness` (`WidgetComponent.GetWidget` (`self.Widget`))))
    (`/Game/Characters/Ai/WB_Alertness.StateManager` _aswb_alertness "Investigate")
    (`SceneComponent.SetVisibility` (`self.Widget`) true true)
    (else
      (`KismetSystemLibrary.PrintString` (`KismetStringLibrary.Conv_DoubleToString` _alertacc) true true (struct :`G` 0.66 :`B` 1.0 :`A` 1.0) 0.01 :!label _label)
      (set `CharacterMovementComponent.MaxWalkSpeed` (`self.SpeedPatrol`) (`self.CharacterMovement`))
      (`SceneComponent.SetVisibility` (`self.Widget`) false true))))

(event `self.ReceiveTick`
  (params (DeltaSeconds :type "Float (single-precision)"))
  (bind _alertacc (`self.AlertAcc`))
  (bind _aswb_alertness (cast `/Game/Characters/Ai/WB_Alertness` (`WidgetComponent.GetWidget` (`self.Widget`))))
  (`/Game/Characters/Ai/WB_Alertness.RadialProgress` _aswb_alertness _alertacc)
  (if (== _alertacc 0.0)
    (goto _label)))

(event `SetStateNormal`
  (goto _label))

(fn `UserConstructionScript`)